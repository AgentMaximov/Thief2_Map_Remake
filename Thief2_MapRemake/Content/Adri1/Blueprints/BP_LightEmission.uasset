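; BP_LightEmission is a point light actor that reports how lit the player character is.
; Each Tick it traces on the Camera channel from the light to the player's mesh.
; A hit distance within the attenuation radius sets BP_PlayerCharacter's LightLevel, scaled linearly up to 16 nearest the light, without checking what was hit.
; The construction script sizes a sphere component to the attenuation radius.
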(event EventTick
  (params (DeltaSeconds :type Float%20%28single-precision%29))
  (bind _pointlight (Variables|Default|GetPointLight))
  (bind _attenuationradius (Variables|/Script/Engine.LocalLightComponent|GetAttenuationRadius _pointlight))
  (bind _outhit (Collision|LineTraceByChannel (Transformation|GetWorldLocation (Variables|Default|GetPointLight)) (Transformation|GetWorldLocation (Variables|/Script/Engine.Character|GetMesh (Game|GetPlayerCharacter 0))) "TraceTypeQuery2" false 0 "None"))
  (if (<= (.distance _outhit) _attenuationradius)
    (Variables|/Game/Blueprints/Player/BP_PlayerCharacter.BP_PlayerCharacter_C|SetLightLevel (.AsBP%20Player%20Character (Utilities|Casting|CastToBP_PlayerCharacter (Game|GetPlayerCharacter 0))) (* (- 1.0 (/ (.distance _outhit) _attenuationradius)) 16.0))))

(fn ConstructionScript
  (Components|Sphere|SetSphereRadius (Variables|Default|GetSphere) (Variables|/Script/Engine.LocalLightComponent|GetAttenuationRadius (Variables|Default|GetPointLight)) true))