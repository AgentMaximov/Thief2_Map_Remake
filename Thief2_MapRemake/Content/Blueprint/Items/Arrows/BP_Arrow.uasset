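; Arrow projectile whose Type decides its effect on impact.
; Tick sweeps it forward by a fixed per-frame step, unscaled by delta time, and a box hit on anything but the shooter applies the effect, then destroys it.
; Water switches off lights, Fire spawns an explosion, Moss patches static meshes, Adam Rope calls the player.
; Rope (wood or fabric only) and Vine trace downward to size a spawned ladder.
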(event OnComponentHit(Box)
  (params (HitComponent :type Primitive%20Component%20Object%20Reference) (OtherActor :type Actor%20Object%20Reference) (OtherComp :type Primitive%20Component%20Object%20Reference) (NormalImpulse :type Vector :default "0, 0, 0") (Hit :type Hit%20Result%20Structure%20%28by%20ref%29))
  (bind (_bblockinghit _binitialoverlap _time _distance _location _impactpoint _normal _impactnormal _physmat _hitactor) (Collision|BreakHitResult Hit))
  (if (not (== OtherActor (Variables|Default|GetShooter)))
    (switch Utilities|FlowControl|Switch|SwitchonE_ArrowType (Variables|Default|GetType)
      (:NewEnumerator0
        _)
      (:NewEnumerator1
        (bind _asbp_light (Utilities|Casting|CastToBP_Light OtherActor)
          (:then
            (Default|Switch _asbp_light true false))
          (:CastFailed
            _)))
      (:NewEnumerator2
        (if (or (== _physmat "/Game/Blueprint/Surfaces/ColorMaterials/M_Bois.M_Bois") (== _physmat "/Game/Blueprint/Surfaces/ColorMaterials/M_Tissu.M_Tissu"))
          (CallFunction|CreateRope _location)))
      (:NewEnumerator3
        (CallFunction|CreateRope _location))
      (:NewEnumerator4
        (if (== (Utilities|GetClass _hitactor) "/Script/Engine.StaticMeshActor")
          (CallFunction|SpawnMoss _location _normal)))
      (:NewEnumerator5
        (CallFunction|ExplodeArrow _location))
      (:NewEnumerator6
        (Default|UseOfRopeArrow (.AsBP%20Player%20Character (Utilities|Casting|CastToBP_PlayerCharacter (Game|GetPlayerCharacter 0))) _location)))
    (Actor|DestroyActor)))

(event Custom|Create%20Rope
  (params (HitLocation :type Vector))
  (bind _outhit (Collision|LineTraceByChannel HitLocation (+ HitLocation "0.000000,0.000000,-1000.000000") "TraceTypeQuery1" false 0 "ForDuration"))
  (if (.bBlockingHit (Collision|BreakHitResult _outhit))
    (if (> (.Distance (Collision|BreakHitResult _outhit)) 1e+02)
      (Development|PrintString "buh")
      (Game|SpawnActorfromClass "/Game/Blueprint/Level-Elements/BP_Ladder.BP_Ladder_C" (Math|Transform|MakeTransform (.Location (Collision|BreakHitResult _outhit))) "Undefined" "MultiplyWithRoot" 0 "0.000000,0.000000,0.000000" (- (Math|Vector|MakeVector 0.0 0.0 (.Distance (Collision|BreakHitResult _outhit))) "0.000000,0.000000,-30.000000") 0))
    (else
      (Development|PrintString (Utilities|String|ToString(Vector) (.Location (Collision|BreakHitResult _outhit))))
      (Game|SpawnActorfromClass "/Game/Blueprint/Level-Elements/BP_Ladder.BP_Ladder_C" (Math|Transform|MakeTransform HitLocation) "Undefined" "MultiplyWithRoot" 0 "0.000000,0.000000,-950.000000" "0.000000,0.000000,0.000000" 0))))

(event Custom|SpawnMoss
  (params (HitLocation :type Vector) (HitNormal :type Vector))
  (Game|SpawnActorfromClass "/Game/Blueprint/Items/Arrows/BP_MossPatch.BP_MossPatch_C" (Math|Transform|MakeTransform HitLocation (Math|Rotator|FindLookatRotation HitLocation (+ HitLocation HitNormal))) "Undefined" "MultiplyWithRoot" 0 0))

(event Custom|ExplodeArrow
  (params (HitLocation :type Vector))
  (Game|SpawnActorfromClass "/Game/Blueprint/Items/Arrows/BP_FireArrowExplosion.BP_FireArrowExplosion_C" (Math|Transform|MakeTransform HitLocation) "Undefined" "MultiplyWithRoot" 0 3e+02 0))

(event EventBeginPlay)

(event Collision|EventActorBeginOverlap
  (params (OtherActor :type Actor%20Object%20Reference)))

(event EventTick
  (params (DeltaSeconds :type Float%20%28single-precision%29))
  (Transformation|SetActorLocation (+ (Transformation|GetActorLocation) (* (Transformation|GetActorForwardVector) (Variables|Default|GetForwardSpeed))) true true))

(fn ConstructionScript)