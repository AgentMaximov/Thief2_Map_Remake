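; Player character Blueprint that handles interaction, quest progress, room tracking and the inventory item widget.
; Capsule overlaps and a per-tick, debug-drawn visibility trace toward the Muzzle both set UsableActor, which ActionInteract messages through BPI_Interact.
; Quest flags are sized from the GameInstance difficulty, and overlapping BP_RoomEnter actors supply the current room for SearchRoom.
; AdjustLightLevel only ever raises the stored light level.
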(event OnComponentBeginOverlap(CapsuleComponent)
  (params (OverlappedComponent :type Primitive%20Component%20Object%20Reference) (OtherActor :type Actor%20Object%20Reference) (OtherComp :type Primitive%20Component%20Object%20Reference) (OtherBodyIndex :type Integer) (bFromSweep :type Boolean) (SweepResult :type Hit%20Result%20Structure%20%28by%20ref%29))
  ;[1 1 1] Detection collission avec objet interactible
  (if (Utilities|DoesObjectImplementInterface OtherActor "/Game/Blueprint/System/Interface/BPI_Interact.BPI_Interact_C")
    (Variables|Default|SetNearUsableObject true)
    (Variables|Default|SetUsableActor OtherActor)))

(event OnComponentEndOverlap(CapsuleComponent)
  (params (OverlappedComponent :type Primitive%20Component%20Object%20Reference) (OtherActor :type Actor%20Object%20Reference) (OtherComp :type Primitive%20Component%20Object%20Reference) (OtherBodyIndex :type Integer))
  ;[1 1 1] Detection collission avec objet interactible
  (if (Utilities|DoesObjectImplementInterface OtherActor "/Game/Blueprint/System/Interface/BPI_Interact.BPI_Interact_C")
    (Variables|Default|SetNearUsableObject false)
    (Variables|Default|SetUsableActor 0)))

(event Custom|ValidQuest
  (params (ID :type Integer))
  (bind _listquestssuccess (Variables|Progress|GetListQuestsSuccess))
  ;[0.9607 1 0.4689] Valide une Quete en fonction de l'ID
  (if (<= ID (Utilities|Array|LastIndex _listquestssuccess))
    (Utilities|Array|SetArrayElem _listquestssuccess ID true)))

(event Custom|SetUpQuest
  ;[1 0.1234 0.4179] Ajuste les quetes en fonction de la difficulté
  (Utilities|Array|Clear (Variables|Progress|GetListQuestsSuccess))
  (bind _asbp_game_instance (Utilities|Casting|CastToBP_GameInstance (Game|GetGameInstance)))
  (for _index (range 1 (Utilities|Array|Get(acopy) (Variables|/Game/Blueprint/BP_GameInstance.BP_GameInstance_C|GetNumberOfObjectivesPerDifficulties _asbp_game_instance) (Variables|/Game/Blueprint/BP_GameInstance.BP_GameInstance_C|GetDifficulty _asbp_game_instance)))
    (Utilities|Array|Add (Variables|Progress|GetListQuestsSuccess) false)))

(event Custom|SelectRoom
  (params (IDRoom :type Integer))
  (bind _allroomvisited (Variables|Progress|GetAllRoomVisited))
  ;[0.6922 1 0.5444] Ajoute une salle a la liste des salle parcourues et selectionne la salle actuelle
  (Variables|Progress|SetCurrentRoom IDRoom)
  (if (not (Utilities|Array|ContainsItem _allroomvisited IDRoom))
    (Utilities|Array|Add _allroomvisited IDRoom)))

(event Custom|ActionInteract
  (bind _usableactor (Variables|Default|GetUsableActor)
    (:then
      (Class|BPIInteract|Interact(Message) _usableactor self))
    (:else)))

(event Custom|Pointer
  (bind (_outhit _returnvalue) (Collision|LineTraceByChannel (Transformation|GetActorLocation) (Transformation|GetWorldLocation (Variables|Default|GetMuzzle)) "TraceTypeQuery1" false 0 "ForDuration" true "(R=1.000000,G=0.000000,B=0.000000,A=1.000000)" "(R=0.000000,G=1.000000,B=0.000000,A=1.000000)" 2.0))
  (if _returnvalue
    (if (Utilities|DoesObjectImplementInterface (.HitActor (Collision|BreakHitResult _outhit)) "/Game/Blueprint/System/Interface/BPI_Interact.BPI_Interact_C")
      (Variables|Default|SetUsableActor (.HitActor (Collision|BreakHitResult _outhit)))
      (else
        (Variables|Default|SetUsableActor 0)))))

(event Custom|SearchRoom
  (bind _capsulecomponent (Variables|Collision|GetCapsuleComponent))
  (bind _overlappingactors (Collision|GetOverlappingActors _capsulecomponent "/Game/Blueprint/Level-Elements/ColisionSpaces/BP_RoomEnter.BP_RoomEnter_C" :!class /Script/Engine.PrimitiveComponent))
  ;[0.4605 1 0.2419] Selectionne une salle ou le joueur est présent sinon met la salle 0
  (if (Utilities|Array|IsNotEmpty _overlappingactors)
    (bind _asbp_room_enter (Utilities|Casting|CastToBP_RoomEnter (Utilities|Array|Get(acopy) _overlappingactors)))
    (CallFunction|SelectRoom (Variables|/Game/Blueprint/Level-Elements/ColisionSpaces/BP_RoomEnter.BP_RoomEnter_C|GetIDRoom _asbp_room_enter))
    (else
      (Variables|Progress|SetCurrentRoom 0))))

(event EventBeginPlay
  (bind _bpc_inventory (Variables|Default|GetBPC_Inventory))
  (bind _asbp_game_mode (Utilities|Casting|CastToBP_GameMode (Game|GetGameMode)))
  (Variables|Default|SetGameMode _asbp_game_mode)
  (bind _asbp_player_controller (Utilities|Casting|CastToBP_PlayerController (Pawn|GetController)))
  (Variables|Default|SetPlayerController _asbp_player_controller)
  (CallFunction|SetUpQuest)
  (bind _returnvalue (UserInterface|CreateWidget "/Game/Blueprint/GUI/WBP_Item.WBP_Item_C" 0 _bpc_inventory (Variables|/Game/Blueprint/Items/BPC_Inventory.BPC_Inventory_C|GetCurrentItem _bpc_inventory)))
  (bind _output_get (Variables|/Game/Blueprint/Items/BPC_Inventory.BPC_Inventory_C|SetItemWidget _bpc_inventory _returnvalue))
  (UserInterface|Viewport|AddtoViewport _output_get 0))

(event EventTick
  (params (DeltaSeconds :type Float%20%28single-precision%29))
  (CallFunction|Pointer))

(fn ConstructionScript)

(fn AdjustLightLevel
  (params (LightSourceLevel :type Float%20%28double-precision%29))
  (Variables|Light|SetLightLevel (Math|Float|SelectFloat LightSourceLevel (Variables|Light|GetLightLevel) (> LightSourceLevel (Variables|Light|GetLightLevel)))))