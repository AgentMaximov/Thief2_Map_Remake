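; Player character Blueprint handling interaction, ladders, ledge climbing, bow display, quest flags and room tracking.
; BeginPlay sizes the quest list by difficulty and creates the inventory item widget.
; Capsule overlaps and a per-tick trace to the muzzle set the usable BPI_Interact actor, while Tick resets the light flag so AdjustLightLevel keeps the brightest source.
; In-development climbing uses stacked traces to estimate ledge height, then a timeline lifts the character.
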(event OnComponentBeginOverlap(CapsuleComponent)
  (params (OverlappedComponent :type Primitive%20Component%20Object%20Reference) (OtherActor :type Actor%20Object%20Reference) (OtherComp :type Primitive%20Component%20Object%20Reference) (OtherBodyIndex :type Integer) (bFromSweep :type Boolean) (SweepResult :type Hit%20Result%20Structure%20%28by%20ref%29))
  ;[1 1 1] Detection collission avec objet interactible
  (if (Utilities|DoesObjectImplementInterface OtherActor "/Game/Blueprint/System/Interface/BPI_Interact.BPI_Interact_C")
    (Variables|Default|SetNearUsableObject true)
    (Variables|Default|SetUsableActor OtherActor)))

(event OnComponentEndOverlap(CapsuleComponent)
  (params (OverlappedComponent :type Primitive%20Component%20Object%20Reference) (OtherActor :type Actor%20Object%20Reference) (OtherComp :type Primitive%20Component%20Object%20Reference) (OtherBodyIndex :type Integer))
  ;[1 1 1] Detection collission avec objet interactible
  (if (Utilities|DoesObjectImplementInterface OtherActor "/Game/Blueprint/System/Interface/BPI_Interact.BPI_Interact_C")
    (Variables|Default|SetNearUsableObject false)
    (Variables|Default|SetUsableActor 0)))

(event Custom|ValidQuest
  (params (ID :type Integer))
  (bind _listquestssuccess (Variables|Progress|GetListQuestsSuccess))
  ;[0.9607 1 0.4689] Valide une Quete en fonction de l'ID
  (if (<= ID (Utilities|Array|LastIndex _listquestssuccess))
    (Utilities|Array|SetArrayElem _listquestssuccess ID true)))

(event Custom|PeutSeHisser
  (bind _returnvalue (Transformation|GetActorLocation))
  (bind _self self)
  (bind _min_climb_height (Variables|Climb|GetMin%20Climb%20Height))
  (bind _mesh (Variables|Character|GetMesh))
  (bind _mesh_2 (Variables|Character|GetMesh))
  (bind _max_climb_height (Variables|Climb|GetMax%20Climb%20Height))
  (bind _mesh_3 (Variables|Character|GetMesh))
  (bind _returnvalue_2 (Transformation|GetWorldLocation _mesh_2))
  (bind (_x _y _z) (Math|Vector|BreakVector _returnvalue))
  (bind _returnvalue_3 (Transformation|GetWorldLocation _mesh))
  (bind _returnvalue_4 (Transformation|GetActorLocation _self))
  (bind _returnvalue_5 (Transformation|GetWorldLocation _mesh_3))
  (bind _returnvalue_6 (+ (.z _returnvalue_3) _min_climb_height))
  (bind _returnvalue_7 (+ (.z _returnvalue_2) _max_climb_height))
  (bind _returnvalue_8 (Math|Vector|MakeVector (.x _returnvalue_2) (.y _returnvalue_2) _returnvalue_7))
  (bind _returnvalue_9 (Math|Vector|MakeVector (.x _returnvalue_3) (.y _returnvalue_3) _returnvalue_6))
  ;[1 0 0.4129] Climbing (en cours de dev)
  ;;[0.3958 0.01962 0.07895] Commence par vérifier s'il y a un plafond
  (bind _returnvalue_10 (Collision|LineTraceByChannel _returnvalue (Math|Vector|MakeVector _x _y (+ _z (Variables|Climb|GetRoof%20Detections))) "TraceTypeQuery1" false 0 "ForDuration"))
  (if (not _returnvalue_10)
    ;;[1 0 0.04677] Lance deux rayons. Le premier à la hauteur minimun de climb et le second juste au dessus de la hauteur maximum. Si le Min touche mais pas le Max, le personnage peut se hisser.
    (bind _returnvalue_11 (Collision|LineTraceByChannel _returnvalue_9 (+ _returnvalue_9 (* (Math|Vector|GetForwardVector (Transformation|GetWorldRotation _mesh)) (Variables|Climb|GetClimb%20Detection))) "TraceTypeQuery1" false 0 "ForDuration"))
    (if _returnvalue_11
      (bind _returnvalue_12 (Collision|LineTraceByChannel _returnvalue_8 (+ _returnvalue_8 (* (Math|Vector|GetForwardVector (Transformation|GetWorldRotation _mesh_2)) 1e+02)) "TraceTypeQuery1" false 0 "ForDuration" true "(R=0.000000,G=0.229393,B=1.000000,A=1.000000)" "(R=0.000000,G=0.971071,B=1.000000,A=1.000000)"))
      (if (not _returnvalue_12)
        (Variables|Climb|SetPrevious%20Self%20Location (Math|Vector|MakeVector (.x _returnvalue_4) (.y _returnvalue_4) (- (.z _returnvalue_4) 18.0)))
        (Variables|Climb|SetPeut%20se%20Hisser true)
        ;;[1 0.3557 0.9521] Empêche de subir des dégâts de chute si on se hisse
        (Variables|FallDamages|SetFall%20Can%20Damage false)
        (Variables|FallDamages|SetTime%20Falling 0.0)
        ;;[1 0.09896 0] Vient vérifier à quelle hauteur on peut se hisser
        (for _index (range 0 (Variables|Climb|GetClimb%20Accuracy))
          (bind _height (CallFunction|FindClimbHeight _index))
          (bind _returnvalue_13 (Collision|LineTraceByChannel (Math|Vector|MakeVector (.x _returnvalue_5) (.y _returnvalue_5) (+ (.z _returnvalue_5) _height)) (+ (Math|Vector|MakeVector (.x _returnvalue_5) (.y _returnvalue_5) (+ (.z _returnvalue_5) _height)) (* (Math|Vector|GetForwardVector (Transformation|GetWorldRotation _mesh_3)) 1e+02)) "TraceTypeQuery1" false 0 "ForDuration" true "(R=0.000000,G=0.229393,B=1.000000,A=1.000000)" "(R=0.000000,G=0.971071,B=1.000000,A=1.000000)"))
          (if _returnvalue_13
            (Math|Integer|IncrementInt (Variables|Climb|GetClimb%20Raycast%20Counter))))
        (bind _height_2 (CallFunction|FindClimbHeight (Variables|Climb|GetClimb%20Raycast%20Counter)))
        (Variables|Climb|SetClimb%20Height _height_2)
        (Variables|Climb|SetClimb%20Raycast%20Counter 0)
        (CallFunction|SeHisser)))))

(event Custom|SetUpQuest
  ;[1 0.1234 0.4179] Ajuste les quetes en fonction de la difficulté
  (Utilities|Array|Clear (Variables|Progress|GetListQuestsSuccess))
  (bind _asbp_game_instance (Utilities|Casting|CastToBP_GameInstance (Game|GetGameInstance)))
  (for _index (range 1 (Utilities|Array|Get(acopy) (Variables|/Game/Blueprint/BP_GameInstance.BP_GameInstance_C|GetNumberOfObjectivesPerDifficulties _asbp_game_instance) (Variables|/Game/Blueprint/BP_GameInstance.BP_GameInstance_C|GetDifficulty _asbp_game_instance)))
    (Utilities|Array|Add (Variables|Progress|GetListQuestsSuccess) false)))

(event Custom|ShowBow
  (params (Show? :type Boolean))
  ;[1 1 1] BOW
  (Development|SetHiddeninGame (Variables|Default|GetBow) (not Show?) true))

(event Custom|SelectRoom
  (params (IDRoom :type Integer))
  (bind _allroomvisited (Variables|Progress|GetAllRoomVisited))
  ;[0.6922 1 0.5444] Ajoute une salle a la liste des salle parcourues et selectionne la salle actuelle
  (Variables|Progress|SetCurrentRoom IDRoom)
  (if (not (Utilities|Array|ContainsItem _allroomvisited IDRoom))
    (Utilities|Array|Add _allroomvisited IDRoom)))

(event Custom|Se%20Hisser
  (bind _previous_self_location (Variables|Climb|GetPrevious%20Self%20Location))
  (bind (_x _y _z) (Math|Vector|BreakVector _previous_self_location))
  ;[1 0 0.4129] Climbing (en cours de dev)
  ;;[0.5463 0 1] Vérifie à quelle hauteur le personnage peut climb et set sa position
  (Variables|Climb|SetCanMove false)
  (Variables|Climb|SetPrevious%20Self%20Rotation (Transformation|GetActorRotation self))
  (Variables|Climb|SetNew%20Position%20%28Climb%29 (Math|Vector|MakeVector _x _y (+ _z (Variables|Climb|GetClimb%20Height) 9e+01)))
  (bind _alpha (Timeline|Chronologie PlayFromStart)
    (:Update
      (Transformation|SetActorLocation self (Math|Vector|Lerp(Vector) (Variables|Climb|GetPrevious%20Self%20Location) (Variables|Climb|GetNew%20Position%20%28Climb%29) _alpha) false false))
    (:Finished
      (Transformation|SetActorLocation self (+ (Variables|Climb|GetNew%20Position%20%28Climb%29) (* (Math|Vector|GetRightVector (Math|Rotator|MakeRotator (.Roll (Math|Rotator|BreakRotator (Variables|Climb|GetPrevious%20Self%20Rotation))) (.Pitch (Math|Rotator|BreakRotator (Variables|Climb|GetPrevious%20Self%20Rotation))) (+ (.Yaw (Math|Rotator|BreakRotator (Variables|Climb|GetPrevious%20Self%20Rotation))) 2.7e+02))) 8e+01)) false false)
      (Variables|Climb|SetPeut%20se%20Hisser false)
      ;;;[1 0.3557 0.9521] Empêche de subir des dégâts de chute si on se hisse
      (Variables|FallDamages|SetFall%20Can%20Damage false)
      (Variables|FallDamages|SetTime%20Falling 0.0)
      (Variables|Climb|SetCanMove true))))

(event Custom|Pointer
  (bind (_outhit _returnvalue) (Collision|LineTraceByChannel (Transformation|GetActorLocation) (Transformation|GetWorldLocation (Variables|Default|GetMuzzle)) "TraceTypeQuery1" false 0 "ForOneFrame" true "(R=1.000000,G=0.000000,B=0.000000,A=1.000000)" "(R=0.000000,G=1.000000,B=0.000000,A=1.000000)" 2.0))
  (if _returnvalue
    (if (Utilities|DoesObjectImplementInterface (.HitActor (Collision|BreakHitResult _outhit)) "/Game/Blueprint/System/Interface/BPI_Interact.BPI_Interact_C")
      (Variables|Default|SetUsableActor (.HitActor (Collision|BreakHitResult _outhit)))
      (else
        (Variables|Default|SetUsableActor 0)))))

(event Custom|SearchRoom
  (bind _capsulecomponent (Variables|Collision|GetCapsuleComponent))
  (bind _overlappingactors (Collision|GetOverlappingActors _capsulecomponent "/Game/Blueprint/Level-Elements/ColisionSpaces/BP_RoomEnter.BP_RoomEnter_C" :!class /Script/Engine.PrimitiveComponent))
  ;[0.4605 1 0.2419] Selectionne une salle ou le joueur est présent sinon met la salle 0
  (if (Utilities|Array|IsNotEmpty _overlappingactors)
    (bind _asbp_room_enter (Utilities|Casting|CastToBP_RoomEnter (Utilities|Array|Get(acopy) _overlappingactors)))
    (CallFunction|SelectRoom (Variables|/Game/Blueprint/Level-Elements/ColisionSpaces/BP_RoomEnter.BP_RoomEnter_C|GetIDRoom _asbp_room_enter))
    (else
      (Variables|Progress|SetCurrentRoom 0))))

(event Custom|UseInteract
  (Development|PrintString "Interaction Attempted" true true "(R=1.000000,G=0.294352,B=0.986959,A=1.000000)")
  (bind _usableactor (Variables|Default|GetUsableActor)
    (:then
      (Class|BPIInteract|Interact(Message) _usableactor self true))
    (:else)))

(event Custom|MoveArrow
  (params (HoldTimer :type Float%20%28double-precision%29))
  ;[1 1 1] BOW
  (Transformation|SetRelativeLocation (Variables|Default|GetArrowMesh) (Math|Vector|Lerp(Vector) "667.782843,-0.459209,3.845727" "-980.000000,-370.000000,-9.000000" (/ HoldTimer 1.5)) false false))

(event Custom|StickToLadder
  (params (Ladder :type BP%20Ladder%20Object%20Reference))
  (bind _charactermovement (Variables|Character|GetCharacterMovement))
  (Variables|Movement|SetCurrentLadder Ladder)
  (Variables|Movement|SetOnLadder true)
  (Variables|/Script/Engine.CharacterMovementComponent|SetGravityScale _charactermovement 0.0)
  (Variables|/Script/Engine.MovementComponent|SetVelocity _charactermovement "0, 0, 0"))

(event Custom|UnstickToLadder
  (Variables|Movement|SetOnLadder false)
  (Variables|/Script/Engine.CharacterMovementComponent|SetGravityScale (Variables|Character|GetCharacterMovement) 1.0))

(event EventBeginPlay
  (bind _bpc_inventory (Variables|Default|GetBPC_Inventory))
  (bind _asbp_game_mode (Utilities|Casting|CastToBP_GameMode (Game|GetGameMode)))
  (Variables|Références|SetGameMode _asbp_game_mode)
  (bind _asbp_player_controller (Utilities|Casting|CastToBP_PlayerController (Pawn|GetController)))
  (Variables|Références|SetPlayerController _asbp_player_controller)
  (CallFunction|SetUpQuest)
  (bind _returnvalue (UserInterface|CreateWidget "/Game/Blueprint/GUI/WBP_Item.WBP_Item_C" 0 _bpc_inventory (Variables|/Game/Blueprint/Items/BPC_Inventory.BPC_Inventory_C|GetCurrentItem _bpc_inventory)))
  (bind _output_get (Variables|/Game/Blueprint/Items/BPC_Inventory.BPC_Inventory_C|SetItemWidget _bpc_inventory _returnvalue))
  (UserInterface|Viewport|AddtoViewport _output_get 0))

(event EventTick
  (params (DeltaSeconds :type Float%20%28single-precision%29))
  ;[1 0.766 0] Event Tick
  (Utilities|FlowControl|Sequence
    (:then_0
      (Variables|Light|SetLightModified false)
      (CallFunction|Pointer)
      (Development|PrintString (Utilities|String|ToString(Float) (Variables|Light|GetLightLevel)) true true "(R=0.000000,G=0.660000,B=1.000000,A=1.000000)" 0.0))))

(fn ConstructionScript)

(fn AdjustLightLevel
  (params (LightSourceLevel :type Float%20%28double-precision%29))
  (if (Variables|Light|GetLightModified)
    (Variables|Light|SetLightLevel (Math|Float|SelectFloat LightSourceLevel (Variables|Light|GetLightLevel) (> LightSourceLevel (Variables|Light|GetLightLevel))))
    (else
      (Variables|Light|SetLightLevel LightSourceLevel))))

(fn FindClimbHeight
  (params (Index :type Integer))
  (return (+ (/ (* (Math|Conversions|ToFloat(Integer) Index) (- (Variables|Climb|GetMax%20Climb%20Height) (Variables|Climb|GetMin%20Climb%20Height))) (Math|Conversions|ToFloat(Integer) (Variables|Climb|GetClimb%20Accuracy))) (Variables|Climb|GetMin%20Climb%20Height))))