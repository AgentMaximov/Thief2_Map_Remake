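; BP_ScoutingOrb is a deployable orb the player can view through to scout, and it switches off BP_Camera actors while they overlap its box.
; It starts with physics on, then freezes when a per-tick sphere trace hits something.
; Interacting hands view and input to the orb, where Look rotates it and the orb action returns to player view.
; After LifeTime it returns to inventory, restores player view and destroys itself.
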(event OnComponentBeginOverlap(Box)
  (params (OverlappedComponent :type Primitive%20Component%20Object%20Reference) (OtherActor :type Actor%20Object%20Reference) (OtherComp :type Primitive%20Component%20Object%20Reference) (OtherBodyIndex :type Integer) (bFromSweep :type Boolean) (SweepResult :type Hit%20Result%20Structure%20%28by%20ref%29))
  (bind _asbp_camera (Utilities|Casting|CastToBP_Camera OtherActor))
  (Default|SwitchOff _asbp_camera))

(event OnComponentEndOverlap(Box)
  (params (OverlappedComponent :type Primitive%20Component%20Object%20Reference) (OtherActor :type Actor%20Object%20Reference) (OtherComp :type Primitive%20Component%20Object%20Reference) (OtherBodyIndex :type Integer))
  (bind _asbp_camera (Utilities|Casting|CastToBP_Camera OtherActor))
  (Default|Switchon _asbp_camera))

(event Custom|Life
  (Utilities|FlowControl|Delay (Variables|Default|GetLifeTime))
  (Default|AddItem (Variables|/Game/Blueprint/Character/BP_PlayerCharacter.BP_PlayerCharacter_C|GetBPC_Inventory (Variables|Default|GetPlayerCharacter)) "/Game/Blueprint/Items/DA_ScoutingOrb.DA_ScoutingOrb" 1)
  (Default|PlayerView (Variables|/Game/Blueprint/Character/BP_PlayerCharacter.BP_PlayerCharacter_C|GetPlayerController (Variables|Default|GetPlayerCharacter)))
  (Actor|DestroyActor))

(event Input|EnhancedActionEvents|EnhancedInputActionIA_ScoutingOrb
  (params (ActionValue :type Boolean) (ElapsedSeconds :type Float%20%28double-precision%29) (TriggeredSeconds :type Float%20%28double-precision%29) (InputAction :type Input%20Action%20Object%20Reference :default "/Game/Blueprint/Input/IA_ScoutingOrb.IA_ScoutingOrb"))
  (:Started
    (Default|PlayerView (Variables|/Game/Blueprint/Character/BP_PlayerCharacter.BP_PlayerCharacter_C|GetPlayerController (Variables|Default|GetPlayerCharacter)))))

(event Input|EnhancedActionEvents|EnhancedInputActionIA_Look
  (params (ActionValue :type Vector%202D%20Structure) (ElapsedSeconds :type Float%20%28double-precision%29) (TriggeredSeconds :type Float%20%28double-precision%29) (InputAction :type Input%20Action%20Object%20Reference :default "/Game/Blueprint/Input/IA_Look.IA_Look"))
  (Transformation|AddRelativeRotation (Variables|Default|GetSphere) (Math|Rotator|MakeRotator 0.0 (- (.y ActionValue) 0.0) (.x ActionValue)) false false))

(event EventInteract
  (params (Player :type BP%20Player%20Character%20Object%20Reference) (IsInteractedByPlayer :type Boolean))
  (bind _returnvalue (Game|GetPlayerController 0))
  (bind _playercontroller (Variables|/Game/Blueprint/Character/BP_PlayerCharacter.BP_PlayerCharacter_C|GetPlayerController Player))
  (Default|ScoutingOrbView _playercontroller self)
  (Input|EnableInput self _returnvalue)
  (Input|DisableInput _playercontroller _returnvalue))

(event EventTick
  (params (DeltaSeconds :type Float%20%28single-precision%29))
  (if (Variables|Default|GetSimulatePhysics)
    (bind _returnvalue (Collision|SphereTraceByChannel (Transformation|GetWorldLocation (Variables|Default|GetSphere)) (Transformation|GetWorldLocation (Variables|Default|GetSphere)) 6e+01 "TraceTypeQuery1" false 0 "ForDuration" true "(R=1.000000,G=0.000000,B=0.000000,A=1.000000)" "(R=0.000000,G=1.000000,B=0.000000,A=1.000000)" 0.1))
    (if _returnvalue
      (Physics|SetSimulatePhysics (Variables|Default|GetSphere) false)
      (Variables|Default|SetSimulatePhysics false))))

(event EventBeginPlay
  (bind _asbp_player_character (Utilities|Casting|CastToBP_PlayerCharacter (Game|GetPlayerCharacter 0)))
  (Variables|Default|SetPlayerCharacter _asbp_player_character)
  (CallFunction|Life)
  (Variables|Default|SetSimulatePhysics true))

(fn ConstructionScript)