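; Switchable torch light that reports how brightly it lights the player character, apparently for stealth detection.
; BeginPlay matches the point light's radius to the detection sphere, whose overlaps track the player.
; While the player is in range, Tick line-traces to their camera offset and sends AdjustLightLevel a clamped, intensity-scaled linear falloff, or zero when blocked.
; Switch toggles the light; water arrows extinguish only open flames, and switching off zeroes the player's light level.
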(event OnComponentBeginOverlap(DetectionCollision)
  (params (OverlappedComponent :type Primitive%20Component%20Object%20Reference) (OtherActor :type Actor%20Object%20Reference) (OtherComp :type Primitive%20Component%20Object%20Reference) (OtherBodyIndex :type Integer) (bFromSweep :type Boolean) (SweepResult :type Hit%20Result%20Structure%20%28by%20ref%29))
  (if (Variables|Default|GetOn)
    (bind _asbp_player_character (Utilities|Casting|CastToBP_PlayerCharacter OtherActor))
    (Utilities|FlowControl|Sequence
      (:then_0
        (Utilities|FlowControl|DoOnce false
          (:Completed
            (Variables|Default|SetPlayer _asbp_player_character))))
      (:then_1
        (Variables|Default|SetPlayerInRange true)))))

(event OnComponentEndOverlap(DetectionCollision)
  (params (OverlappedComponent :type Primitive%20Component%20Object%20Reference) (OtherActor :type Actor%20Object%20Reference) (OtherComp :type Primitive%20Component%20Object%20Reference) (OtherBodyIndex :type Integer))
  (if (Variables|Default|GetOn)
    (Utilities|Casting|CastToBP_PlayerCharacter OtherActor)
    (Variables|Default|SetPlayerInRange false)))

(event EventBeginPlay
  (bind _detectioncollision (Variables|Default|GetDetectionCollision))
  (Rendering|Lighting|SetAttenuationRadius (Variables|Default|GetPointLight) (* (.z (Transformation|GetWorldScale _detectioncollision)) (Variables|/Script/Engine.SphereComponent|GetSphereRadius _detectioncollision) 1.0))
  (if (Variables|Default|GetOn)
    (Rendering|Components|Light|SetIntensity (Variables|Default|GetPointLight) (Variables|Default|GetIntensity))
    (else
      (Rendering|Components|Light|SetIntensity (Variables|Default|GetPointLight) 0.0))))

(event EventTick
  (params (DeltaSeconds :type Float%20%28single-precision%29))
  (bind _player (Variables|Default|GetPlayer))
  (bind _pointlight (Variables|Default|GetPointLight))
  (bind _player_2 (Variables|Default|GetPlayer))
  (if (Variables|Default|GetPlayerInRange)
    (bind _outhit (Collision|LineTraceByChannel (Transformation|GetActorLocation) (+ (Transformation|GetActorLocation _player_2) (Variables|/Game/Blueprint/Character/BP_PlayerCharacter.BP_PlayerCharacter_C|GetCameraOffset _player_2)) "TraceTypeQuery1" false 0 "ForDuration" true "(R=0.993651,G=1.000000,B=0.967060,A=1.000000)" "(R=0.000000,G=1.000000,B=0.000000,A=1.000000)" 0.1))
    (Default|AdjustLightLevel (Variables|Default|GetPlayer) (Math|Float|Clamp(Float) (Math|Float|SelectFloat 0.0 (* (- 1.0 (/ (Math|Vector|Distance(Vector) (Transformation|GetActorLocation) (+ (Transformation|GetActorLocation _player) (Variables|/Game/Blueprint/Character/BP_PlayerCharacter.BP_PlayerCharacter_C|GetCameraOffset _player))) (Variables|/Script/Engine.LocalLightComponent|GetAttenuationRadius _pointlight))) (Variables|/Script/Engine.LightComponentBase|GetIntensity _pointlight) 4.0) (.bBlockingHit (Collision|BreakHitResult _outhit))) 0.0 15.0))))

(fn ConstructionScript)

(fn Switch
  (params (WaterArrow :type Boolean) (Turn%20on? :type Boolean))
  (if Turn%20on?
    (Variables|Default|SetOn true)
    (CallFunction|On/Off (Variables|Default|GetOn) :!label _label)
    (elif WaterArrow
      (if (Variables|Default|GetOpenFlame)
        (Variables|Default|SetOn false)
        (goto _label))
      (else
        (Variables|Default|SetOn false)
        (goto _label)))))

(fn On/Off
  (params (On :type Boolean))
  (bind _pointlight (Variables|Default|GetPointLight))
  (if On
    (Rendering|Components|Light|SetIntensity _pointlight (Variables|Default|GetIntensity))
    (for _array_element (Collision|GetOverlappingActors (Variables|Default|GetDetectionCollision) "/Game/Blueprint/Character/BP_PlayerCharacter.BP_PlayerCharacter_C" :!class /Script/Engine.PrimitiveComponent)
      (Utilities|IsValid _array_element
        (:Is%20Valid
          (Utilities|IsValid (Variables|Default|GetPlayer)
            (:Is%20Valid
              _)
            (:Is%20Not%20Valid
              (Variables|Default|SetPlayer (.AsBP%20Player%20Character (Utilities|Casting|CastToBP_PlayerCharacter _array_element)))))
          (Variables|Default|SetPlayerInRange true))))
    (else
      (Rendering|Components|Light|SetIntensity _pointlight 0.0)
      (Variables|Default|SetPlayerInRange false)
      (Default|AdjustLightLevel (Variables|Default|GetPlayer) 0.0))))