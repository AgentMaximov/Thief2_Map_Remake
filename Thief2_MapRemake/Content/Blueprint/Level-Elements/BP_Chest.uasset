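; BP_Chest is an interactable, optionally locked chest that gives the player money and items when opened.
; Lock modes are none, a single key ID, or a set or random sequence of key IDs, generated at BeginPlay when random or left empty.
; Interact checks the held item's KeyID against the lock, consuming matching sequence entries one per interaction.
; Success and failure play sounds, and the handle rotates to reflect the remaining sequence length.
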(event Custom|InteractSucessful
  (Audio|PlaySoundatLocation (Variables|System|GetPickSucess) (Transformation|GetActorLocation) "0, 0, 0" 1.0 1.0 0.0 0 0 0 0))

(event Custom|InteractNonSucessful
  (Audio|PlaySoundatLocation (Variables|System|GetPickFail) (Transformation|GetActorLocation) "0, 0, 0" 1.0 1.0 0.0 0 0 0 0))

(event EventBeginPlay
  ;[0.01569 1 0] Do not delete
  (if (or (and (Utilities|Enum|Equal(Enum) (Variables|Settings|GetLockMode) "NewEnumerator1") (== (Utilities|Array|Length (Variables|Settings|GetArraySeq)) 0)) (Utilities|Enum|Equal(Enum) (Variables|Settings|GetLockMode) "NewEnumerator0"))
    (for _index (range 1 (Math|Random|RandomIntegerinRange 1 3))
      (Utilities|Array|Add (Variables|Settings|GetArraySeq) (Math|Random|RandomIntegerinRange 1 2)))))

(event EventInteract
  (params (Player :type BP%20Player%20Character%20Object%20Reference) (IsInteractedByPlayer :type Boolean))
  (bind _bpc_inventory (Variables|/Game/Blueprint/Character/BP_PlayerCharacter.BP_PlayerCharacter_C|GetBPC_Inventory Player))
  (bind _currentitem (Variables|/Game/Blueprint/Items/BPC_Inventory.BPC_Inventory_C|GetCurrentItem _bpc_inventory))
  (bind _keyid (Variables|/Game/Blueprint/Items/PDA_Item.PDA_Item_C|GetKeyID _currentitem))
  ;[0.01569 1 0] Lockpicking Logic
  (switch Utilities|FlowControl|Switch|SwitchonELockPossible (Variables|Settings|GetLockMode)
    (:NewEnumerator3
      ;;[0 0.06667 1] Not locked
      (CallFunction|InteractSucessful)
      (CallFunction|IntactedwithDoors Player))
    (:NewEnumerator0
      (bind (_sucessful_ _hasopened_) (CallFunction|TryLockping _keyid :!label _label))
      (if _hasopened_
        ;;[0 0.06667 1] ArraySeq is empty, which mean the lockpick is done
        (CallFunction|InteractSucessful)
        (CallFunction|IntactedwithDoors Player)
        (Variables|Settings|SetLockMode "NewEnumerator3")
        (CallFunction|UpdateHandlePosition)
        (elif _sucessful_
          (CallFunction|InteractSucessful)
          (CallFunction|UpdateHandlePosition)
          (else
            (CallFunction|InteractNonSucessful)))))
    (:NewEnumerator1
      (goto _label))
    (:NewEnumerator2
      ;;[0 0.06667 1] Custom Key
      (if (== _keyid (Variables|Settings|GetKeyID))
        (CallFunction|InteractSucessful)
        (CallFunction|IntactedwithDoors Player)
        (Variables|Settings|SetLockMode "NewEnumerator3")
        (else
          (CallFunction|InteractNonSucessful))))))

(fn ConstructionScript)

(fn IntactedwithDoors
  (params (Player :type BP%20Player%20Character%20Object%20Reference%20%28by%20ref%29))
  (Variables|/Game/Blueprint/Character/BP_PlayerCharacter.BP_PlayerCharacter_C|SetMoney Player (+ (Variables|/Game/Blueprint/Character/BP_PlayerCharacter.BP_PlayerCharacter_C|GetMoney Player) (Variables|Rewards|GetMoney)))
  (for _array_element (Variables|Rewards|GetItems)
    (Default|AddItem (Variables|/Game/Blueprint/Character/BP_PlayerCharacter.BP_PlayerCharacter_C|GetBPC_Inventory Player) (.item _array_element) (.quantity _array_element))
    (Utilities|Array|Clear (Variables|Rewards|GetItems))))

(fn TryLockping
  (params (Held%20Key%20ID :type Integer))
  (bind _arrayseq (Variables|Settings|GetArraySeq))
  (bind _returnvalue (Utilities|Array|Length _arrayseq))
  (bind _returnvalue_2 (== _returnvalue 0))
  (Development|PrintText (Utilities|Text|FormatText "Held Id: {A} 
Wanted Id: {B} 
" Held%20Key%20ID (Utilities|Array|Get(acopy) (Variables|Settings|GetArraySeq))))
  (if (== Held%20Key%20ID (Utilities|Array|Get(acopy) (Variables|Settings|GetArraySeq)))
    (Utilities|Array|RemoveIndex (Variables|Settings|GetArraySeq))
    (return true _returnvalue_2)
    (else
      (return false _returnvalue_2))))

(fn UpdateHandlePosition
  (switch int (Utilities|Array|Length (Variables|Settings|GetArraySeq))
    (:0
      (Variables|Default|SetAngleToSet 9e+01))
    (:1
      (Variables|Default|SetAngleToSet 6e+01))
    (:2
      (Variables|Default|SetAngleToSet 3e+01)))
  (Transformation|SetWorldRotation (Variables|Default|GetPoignee) (Math|Rotator|MakeRotator 0.0 (Variables|Default|GetAngleToSet) 0.0) false false))