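; Interactive door that players and AI swing open or closed with timelines, choosing the opening direction from a front collision overlap.
; Player interaction respects the lock mode (none, key ID, or a set or random pick sequence), while AI bypasses locks.
; Lockpicking consumes the sequence as held item IDs match, turning the handles to show progress and playing success or failure sounds.
; Random sequences, and empty set ones, are filled at BeginPlay.
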(event Custom|InteractSucessful
  (Audio|PlaySoundatLocation (Variables|System|GetPickSucess) (Transformation|GetActorLocation) "0, 0, 0" 1.0 1.0 0.0 0 0 0 0))

(event Custom|InteractNonSucessful
  (Audio|PlaySoundatLocation (Variables|System|GetPickFail) (Transformation|GetActorLocation) "0, 0, 0" 1.0 1.0 0.0 0 0 0 0))

(event Custom|UpdateHandlePosition
  ;[0.01569 1 0] Update Handle Rotation to Match Seq
  (switch int (Utilities|Array|Length (Variables|Settings|GetArraySeq))
    (:0
      (Variables|Default|SetAngleToSet 9e+01))
    (:1
      (Variables|Default|SetAngleToSet 6e+01))
    (:2
      (Variables|Default|SetAngleToSet 3e+01)))
  (Transformation|SetWorldRotation (Variables|Default|GetMeshPoignee) (Math|Rotator|MakeRotator 0.0 (Variables|Default|GetAngleToSet) 0.0) false false)
  (Transformation|SetWorldRotation (Variables|Default|GetMeshPoignee1) (Math|Rotator|MakeRotator 0.0 (Variables|Default|GetAngleToSet) 0.0) false false))

(event Custom|IntactedWithDoors
  (params (CalledByPlayer :type Boolean))
  ;[0.01569 1 0] FlipFlop
  (if (Variables|System|GetisOpen)
    (CallFunction|CloseDoorEvent)
    (else
      (CallFunction|OpenDoorEvent CalledByPlayer))))

(event Custom|CloseDoorEvent
  ;[0.01569 1 0] Will work regardless of who interact for  closure
  (CallFunction|StopOpenLoop)
  (Variables|System|SetisOpen false)
  (Variables|System|SetStartingRotForClose (Transformation|GetActorRotation))
  (bind _alpha (Timeline|Timeline_1 PlayFromStart)
    (:Update
      (Transformation|SetActorRotation (Math|Rotator|Lerp(Rotator) (Variables|System|GetStartingRotForClose) (Variables|System|GetClosedRotation) _alpha true)))))

(event Custom|StopClosingLoop
  ;[0.01569 1 0] Will work regardless of who interact for  closure
  ;;[0.8196 0.2196 1] Avoid duplicate anim
  (bind _alpha (Timeline|Timeline_1 Stop)
    (:Update
      (Transformation|SetActorRotation (Math|Rotator|Lerp(Rotator) (Variables|System|GetStartingRotForClose) (Variables|System|GetClosedRotation) _alpha true)))))

(event Custom|StopOpenLoop
  (bind _closedrotation (Variables|System|GetClosedRotation))
  (bind _closedrotation_2 (Variables|System|GetClosedRotation))
  ;[0.01569 1 0] Opening Process, Should work regardless who interact, PM adamriondy on discord if problems
  ;;[0.8196 0.2196 1] Avoid duplicate anim
  (Utilities|FlowControl|Sequence
    (:then_0
      ;;[0 0.06667 1] Player
      (bind _alpha (Timeline|Timeline_0 Stop)
        (:Update
          (Transformation|SetActorRotation (Math|Rotator|Lerp(Rotator) (Variables|System|GetClosedRotation) (Math|Rotator|MakeRotator (.roll _closedrotation_2) (.pitch _closedrotation_2) (+ (.yaw _closedrotation_2) (stale Custom|OpenDoorEvent _angle))) _alpha)))))
    (:then_1
      ;;[0 0.06667 1] AI
      (bind _alpha_2 (Timeline|Timeline Stop)
        (:Update
          (Transformation|SetActorRotation (Math|Rotator|Lerp(Rotator) (Variables|System|GetClosedRotation) (Math|Rotator|MakeRotator (.roll _closedrotation) (.pitch _closedrotation) (+ (.yaw _closedrotation) (stale Custom|OpenDoorEvent _angle_2))) _alpha_2)))))))

(event Custom|OpenDoorEvent
  (params (IsPlayerInteracted :type Boolean))
  (bind _closedrotation (Variables|System|GetClosedRotation))
  (bind _closedrotation_2 (Variables|System|GetClosedRotation))
  ;[0.01569 1 0] Opening Process, Should work regardless who interact, PM adamriondy on discord if problems
  (CallFunction|StopClosingLoop)
  (Variables|System|SetisOpen true)
  (if IsPlayerInteracted
    (bind _angle (CallFunction|GiveOpeningAngle true))
    ;;[0 0.06667 1] Player
    (bind _alpha (Timeline|Timeline_0 PlayFromStart)
      (:Update
        (Transformation|SetActorRotation (Math|Rotator|Lerp(Rotator) (Variables|System|GetClosedRotation) (Math|Rotator|MakeRotator (.roll _closedrotation_2) (.pitch _closedrotation_2) (+ (.yaw _closedrotation_2) _angle)) _alpha))))
    (else
      (bind _angle_2 (CallFunction|GiveOpeningAngle false))
      ;;[0 0.06667 1] AI
      (bind _alpha_2 (Timeline|Timeline PlayFromStart)
        (:Update
          (Transformation|SetActorRotation (Math|Rotator|Lerp(Rotator) (Variables|System|GetClosedRotation) (Math|Rotator|MakeRotator (.roll _closedrotation) (.pitch _closedrotation) (+ (.yaw _closedrotation) _angle_2)) _alpha_2)))))))

(event EventBeginPlay
  ;[0.01569 1 0] Do not delete
  (Variables|System|SetClosedRotation (Transformation|GetActorRotation))
  (if (or (and (Utilities|Enum|Equal(Enum) (Variables|Settings|GetLockMode) "NewEnumerator1") (== (Utilities|Array|Length (Variables|Settings|GetArraySeq)) 0)) (Utilities|Enum|Equal(Enum) (Variables|Settings|GetLockMode) "NewEnumerator0"))
    (for _index (range 1 (Math|Random|RandomIntegerinRange 1 3))
      (Utilities|Array|Add (Variables|Settings|GetArraySeq) (Math|Random|RandomIntegerinRange 1 2)))))

(event EventInteract
  (params (Player :type BP%20Player%20Character%20Object%20Reference) (IsInteractedByPlayer :type Boolean))
  (bind _bpc_inventory (Variables|/Game/Blueprint/Character/BP_PlayerCharacter.BP_PlayerCharacter_C|GetBPC_Inventory Player))
  (bind _currentitem (Variables|/Game/Blueprint/Items/BPC_Inventory.BPC_Inventory_C|GetCurrentItem _bpc_inventory))
  (bind _keyid (Variables|/Game/Blueprint/Items/PDA_Item.PDA_Item_C|GetKeyID _currentitem))
  ;[0.01569 1 0] Lockpicking Logic
  ;;[0 0.06667 1] If opened by AI, locking state is irrelevalant
  (if IsInteractedByPlayer
    (switch Utilities|FlowControl|Switch|SwitchonELockPossible (Variables|Settings|GetLockMode)
      (:NewEnumerator3
        ;;[0 0.06667 1] Not locked
        (CallFunction|InteractSucessful)
        (CallFunction|IntactedwithDoors true))
      (:NewEnumerator0
        (bind (_sucessful_ _hasopened_) (CallFunction|TryLockping _keyid :!label _label))
        (if _hasopened_
          ;;[0 0.06667 1] ArraySeq is empty, which mean the lockpick is done
          (CallFunction|InteractSucessful)
          (CallFunction|IntactedwithDoors true)
          (Variables|Settings|SetLockMode "NewEnumerator3")
          (CallFunction|UpdateHandlePosition)
          (elif _sucessful_
            (CallFunction|InteractSucessful)
            (CallFunction|UpdateHandlePosition)
            (else
              (CallFunction|InteractNonSucessful)))))
      (:NewEnumerator1
        (goto _label))
      (:NewEnumerator2
        ;;[0 0.06667 1] Custom Key
        (if (== _keyid (Variables|Settings|GetKeyID))
          (CallFunction|InteractSucessful)
          (CallFunction|IntactedwithDoors true)
          (Variables|Settings|SetLockMode "NewEnumerator3")
          (else
            (CallFunction|InteractNonSucessful)))))
    (else
      ;;[0 0.06667 1] AI
      (CallFunction|InteractSucessful)
      (CallFunction|IntactedwithDoors false))))

(fn ConstructionScript)

(fn GiveOpeningAngle
  (params (PlayerInteracted? :type Boolean))
  (if PlayerInteracted?
    (if (Collision|IsOverlappingActor (Variables|Default|GetFrontColl) (Game|GetPlayerCharacter 0) :!class /Script/Engine.PrimitiveComponent)
      (return -9e+01)
      (else
        (return 9e+01)))
    (else
      ;[1 1 1] Checking if not here, so no need to inverse
      (if (Utilities|Array|IsEmpty (Collision|GetOverlappingActors (Variables|Default|GetFrontColl) "/Game/Blueprint/Enemis/EnemyAI/BP_Enemy.BP_Enemy_C" :!class /Script/Engine.PrimitiveComponent))
        (return -9e+01)
        (else
          (return 9e+01))))))

(fn TryLockping
  (params (Held%20Key%20ID :type Integer))
  (bind _arrayseq (Variables|Settings|GetArraySeq))
  (bind _returnvalue (Utilities|Array|Length _arrayseq))
  (bind _returnvalue_2 (== _returnvalue 0))
  (Development|PrintText (Utilities|Text|FormatText "Held Id: {A} 
Wanted Id: {B} 
" Held%20Key%20ID (Utilities|Array|Get(acopy) (Variables|Settings|GetArraySeq))))
  (if (== Held%20Key%20ID (Utilities|Array|Get(acopy) (Variables|Settings|GetArraySeq)))
    (Utilities|Array|RemoveIndex (Variables|Settings|GetArraySeq))
    (return true _returnvalue_2)
    (else
      (return false _returnvalue_2))))