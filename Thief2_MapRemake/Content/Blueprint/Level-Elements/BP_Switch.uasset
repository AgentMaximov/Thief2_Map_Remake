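; BP_Switch is an interactable level switch that toggles its linked cameras off and on.
; Interact alternates through a FlipFlop, calling SwitchOff or SwitchOn on each LinkedCamera entry; the matching LinkedLight loops are still empty.
; A timeline, played forward or reversed, lerps the top and bottom buttons to opposite heights, with CanMove blocking further input until it finishes.
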(event Custom|SwitchOffCamera
  ;[0 0.6875 1] Eteint toutes les tourelles et / ou lights qui sont liées à cet interrupteur
  (for _array_element (Variables|Default|GetLinked%20Camera)
    (Default|SwitchOff _array_element)))

(event Custom|Activation)

(event Custom|Move%20Switches
  (bind _position_02 (Variables|Default|GetPosition_02))
  (bind _position_01 (Variables|Default|GetPosition_01))
  (bind _returnvalue (Math|Vector|MakeVector 0.0 0.0 _position_02))
  (bind _returnvalue_2 (Math|Vector|MakeVector 0.0 0.0 _position_01))
  ;[1 0.7367 0] Movement de l'interrupteur
  (bind _alpha (Timeline|Movement%20Interrupteur PlayFromStart)
    (:Update
      (Utilities|FlowControl|Sequence
        (:then_0
          (Transformation|SetRelativeLocation (Variables|Default|GetButtonTop) (Math|Vector|Lerp(Vector) _returnvalue_2 _returnvalue _alpha) false false))
        (:then_1
          (Transformation|SetRelativeLocation (Variables|Default|GetButtonBottom) (Math|Vector|Lerp(Vector) _returnvalue _returnvalue_2 _alpha) false false))))
    (:Finished
      (Variables|Default|SetCan%20Move true))))

(event Custom|Invert%20Move%20Switches
  (bind _position_02 (Variables|Default|GetPosition_02))
  (bind _position_01 (Variables|Default|GetPosition_01))
  (bind _returnvalue (Math|Vector|MakeVector 0.0 0.0 _position_02))
  (bind _returnvalue_2 (Math|Vector|MakeVector 0.0 0.0 _position_01))
  ;[1 0.7367 0] Movement de l'interrupteur
  (bind _alpha (Timeline|Movement%20Interrupteur ReverseFromEnd)
    (:Update
      (Utilities|FlowControl|Sequence
        (:then_0
          (Transformation|SetRelativeLocation (Variables|Default|GetButtonTop) (Math|Vector|Lerp(Vector) _returnvalue_2 _returnvalue _alpha) false false))
        (:then_1
          (Transformation|SetRelativeLocation (Variables|Default|GetButtonBottom) (Math|Vector|Lerp(Vector) _returnvalue _returnvalue_2 _alpha) false false))))
    (:Finished
      (Variables|Default|SetCan%20Move true))))

(event Custom|SwitchOnCamera
  ;[1 0 0.5102] Allume toutes les camera et / ou light liées à cet interrupteur
  (for _array_element (Variables|Default|GetLinked%20Camera)
    (Default|Switchon _array_element)))

(event Custom|SwitchOnLight
  ;[1 0 0.5102] Allume toutes les camera et / ou light liées à cet interrupteur
  (for _array_element (Variables|Default|GetLinked%20Light)
    _))

(event Custom|SwitchOffLight
  ;[0 0.6875 1] Eteint toutes les tourelles et / ou lights qui sont liées à cet interrupteur
  (for _array_element (Variables|Default|GetLinked%20Light)
    _))

(event EventInteract
  (params (Player :type BP%20Player%20Character%20Object%20Reference) (IsInteractedByPlayer :type Boolean))
  ;[0.517 0.2034 1] Activation / Désactivation
  (if (Variables|Default|GetCan%20Move)
    (Variables|Default|SetCan%20Move false)
    (Utilities|FlowControl|FlipFlop
      (:A
        (CallFunction|SwitchOffCamera)
        (CallFunction|SwitchOffLight)
        (CallFunction|MoveSwitches))
      (:B
        (CallFunction|SwitchonCamera)
        (CallFunction|SwitchonLight)
        (CallFunction|InvertMoveSwitches)))))

(fn ConstructionScript)