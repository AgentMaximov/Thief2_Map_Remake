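; BP_ExfiltrationPoint is a level exit that ends the game when the player enters it with enough completed quests.
; On actor overlap, it casts the other actor to BP_PlayerCharacter and counts the true entries in its ListQuestsSuccess.
; It compares that count to the QuestNeededPerDifficulty entry for the game instance's difficulty, then calls EndGame on BP_GameInstance if the threshold is met.
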(event Collision|EventActorBeginOverlap
  (params (OtherActor :type Actor%20Object%20Reference))
  ;[1 1 1] Verify si le joueur a acomplis un certain nombre de quete pour terminer le niveau
  (bind _asbp_player_character (Utilities|Casting|CastToBP_PlayerCharacter OtherActor))
  (bind _asbp_game_instance (Utilities|Casting|CastToBP_GameInstance (Game|GetGameInstance)))
  (Variables|Default|SetNumberValidQuest 0)
  (for _array_element (Variables|/Game/Blueprint/Character/BP_PlayerCharacter.BP_PlayerCharacter_C|GetListQuestsSuccess _asbp_player_character)
    (if _array_element
      (Math|Integer|IncrementInt (Variables|Default|GetNumberValidQuest))))
  (if (>= (Variables|Default|GetNumberValidQuest) (Utilities|Array|Get(acopy) (Variables|Default|GetQuestNeededPerDifficulty) (Variables|/Game/Blueprint/BP_GameInstance.BP_GameInstance_C|GetDifficulty _asbp_game_instance)))
    (Default|EndGame _asbp_game_instance)))

(fn ConstructionScript)