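; BP_Elevator_Switch is a level button that, on Interact, sends its linked elevator to the switch's Destination.
; Interact plays a press animation, nudging the Button component along local X and back with two timed MoveComponentTo calls.
; It looks up BP_Elevator actors but compares its ID only with the first one found, then stores and activates that elevator on a match.
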(event Custom|AnimButton
  (bind _button (Variables|Default|GetButton))
  (bind _relativelocation (Variables|/Script/Engine.SceneComponent|GetRelativeLocation _button))
  (Components|MoveComponentTo _button (+ _relativelocation "-5.000000,0.000000,0.000000") "0, 0, 0" false false 0.25 false)
  (Components|MoveComponentTo _button (+ _relativelocation "5.000000,0.000000,0.000000") "0, 0, 0" false false 0.25 false))

(event EventBeginPlay)

(event Collision|EventActorBeginOverlap
  (params (OtherActor :type Actor%20Object%20Reference)))

(event EventTick
  (params (DeltaSeconds :type Float%20%28single-precision%29)))

(event EventInteract
  (params (Player :type BP%20Player%20Character%20Object%20Reference))
  (CallFunction|AnimButton)
  (bind _outactors (Actor|GetAllActorsOfClass "/Game/Blueprint/Level-Elements/BP_Elevator.BP_Elevator_C"))
  (if (== (Variables|Default|GetID) (Variables|/Game/Blueprint/Level-Elements/BP_Elevator.BP_Elevator_C|GetID (Utilities|Array|Get(acopy) _outactors)))
    (bind _output_get (Variables|Default|SetLinkedElevator (Utilities|Array|Get(acopy) _outactors)))
    (Default|ActivateElevator _output_get (Variables|Default|GetDestination))))

(fn ConstructionScript)