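; Climbable ladder actor that attaches the player character to itself while the player is inside its trigger box.
; On BeginPlay it converts its top and bottom offsets to world positions, sets the box's half-height from their distance and moves the actor to their midpoint.
; Box overlaps call StickToLadder on BP_PlayerCharacter with the ladder reference on entry and UnstickToLadder on exit.
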(event OnComponentBeginOverlap(Box)
  (params (OverlappedComponent :type Primitive%20Component%20Object%20Reference) (OtherActor :type Actor%20Object%20Reference) (OtherComp :type Primitive%20Component%20Object%20Reference) (OtherBodyIndex :type Integer) (bFromSweep :type Boolean) (SweepResult :type Hit%20Result%20Structure%20%28by%20ref%29))
  (bind _asbp_player_character (Utilities|Casting|CastToBP_PlayerCharacter OtherActor))
  (Default|SticktoLadder _asbp_player_character self))

(event OnComponentEndOverlap(Box)
  (params (OverlappedComponent :type Primitive%20Component%20Object%20Reference) (OtherActor :type Actor%20Object%20Reference) (OtherComp :type Primitive%20Component%20Object%20Reference) (OtherBodyIndex :type Integer))
  (bind _asbp_player_character (Utilities|Casting|CastToBP_PlayerCharacter OtherActor))
  (Default|UnsticktoLadder _asbp_player_character))

(event EventBeginPlay
  (bind _returnvalue (Transformation|GetActorLocation))
  (bind _box (Variables|Default|GetBox))
  (bind _boxextent (Variables|/Script/Engine.BoxComponent|GetBoxExtent _box))
  (Variables|Default|SetPositionBottom (+ (Variables|Default|GetPositionBottom) _returnvalue))
  (Variables|Default|SetPositionTop (+ (Variables|Default|GetPositionTop) _returnvalue))
  (Components|Box|SetBoxExtent _box (Math|Vector|MakeVector (.x _boxextent) (.y _boxextent) (/ (Math|Vector|Distance(Vector) (Variables|Default|GetPositionTop) (Variables|Default|GetPositionBottom)) 2.0)) true)
  (Transformation|SetActorLocation (Math|Vector|Lerp(Vector) (Variables|Default|GetPositionTop) (Variables|Default|GetPositionBottom) 0.5) false false))

(event Collision|EventActorBeginOverlap
  (params (OtherActor :type Actor%20Object%20Reference)))

(event EventTick
  (params (DeltaSeconds :type Float%20%28single-precision%29)))

(fn ConstructionScript)