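; BP_MetalCeiling is a level-element Blueprint that records the horizontal area covered by its Box component.
; On BeginPlay it computes world-space min and max pairs into BoundsX and BoundsY from the box's location, extent and scale, ignoring rotation.
; Overlap, Tick and the construction script are empty, and nothing in this Blueprint reads the stored bounds.
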(event EventBeginPlay
  (bind _box (Variables|Default|GetBox))
  (bind _box_2 (Variables|Default|GetBox))
  (bind _returnvalue (Transformation|GetWorldLocation _box))
  (bind _returnvalue_2 (Transformation|GetWorldLocation _box_2))
  (bind _returnvalue_3 (Transformation|GetWorldScale _box_2))
  (bind _returnvalue_4 (Transformation|GetWorldScale _box))
  (bind _boxextent (Variables|/Script/Engine.BoxComponent|GetBoxExtent _box))
  (bind _boxextent_2 (Variables|/Script/Engine.BoxComponent|GetBoxExtent _box_2))
  (bind _returnvalue_5 (* (.x _boxextent_2) (.x _returnvalue_3)))
  (bind _returnvalue_6 (* (.y _boxextent) (.y _returnvalue_4)))
  (Variables|Default|SetBoundsX (Math|Vector2D|MakeVector2D (- (.x _returnvalue_2) _returnvalue_5) (+ (.x _returnvalue_2) _returnvalue_5)))
  (Variables|Default|SetBoundsY (Math|Vector2D|MakeVector2D (- (.y _returnvalue) _returnvalue_6) (+ (.y _returnvalue) _returnvalue_6))))

(event Collision|EventActorBeginOverlap
  (params (OtherActor :type Actor%20Object%20Reference)))

(event EventTick
  (params (DeltaSeconds :type Float%20%28single-precision%29)))

(fn ConstructionScript)