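; Enemy security camera Blueprint, apparently adapted from a turret, that sweeps between two yaw limits and detects the player through PawnSensing.
; Tick drives the lerped sweep until a sighting stops it, then times how long the player stays unseen to trigger a return to routine.
; Switch events pause or resume it and flip emissive materials.
; Target following, linked-turret alerts and unsee handling are stubs, with related logic left disconnected.
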(event OnSeePawn(PawnSensing)
  (params (Pawn :type Pawn%20Object%20Reference))
  ;[0.4629 1 0] On See Pawn
  ;;[0 1 0.2431] Vérifie si ce que la Camera voit le PJ
  (Utilities|Casting|CastToBP_PlayerCharacter Pawn)
  (Variables|Detection|SetDeltaTimeStandBy 0.0)
  (if (not (Variables|Detection|GetIs%20Targeting))
    (CallFunction|SeePawn Pawn)))

(event Custom|Auto%20Rotation
  (params (Delta%20Time :type Float%20%28double-precision%29))
  (bind _basic_rotaion (Variables|CameraMovement|GetBasic%20Rotaion))
  (bind _basic_rotaion_2 (Variables|CameraMovement|GetBasic%20Rotaion))
  (bind _basic_rotaion_3 (Variables|CameraMovement|GetBasic%20Rotaion))
  ;[0 1 0.4134] Auto Rotation
  (Variables|CameraMovement|SetMoving true)
  (Variables|CameraMovement|SetCurrent%20Lerp (+ (* Delta%20Time (Variables|CameraMovement|GetRotation%20Speed)) (Variables|CameraMovement|GetCurrent%20Lerp)))
  (if (Variables|CameraMovement|GetBackingToRoutine)
    ;;[0 0.6366 1] Revient à sa routine quand le joueur est perdu de vu
    (Transformation|SetActorRotation (Math|Rotator|Lerp(Rotator) (Variables|CameraMovement|GetPrevious%20Self%20Rotation) (Math|Rotator|MakeRotator (.roll _basic_rotaion_2) (.pitch _basic_rotaion_2) (Variables|CameraMovement|GetEnd%20Routine)) (Variables|CameraMovement|GetCurrent%20Lerp)))
    (else
      ;;[0.4662 0 1] Routine de la tourelle.
      (if (Variables|CameraMovement|GetNegate%20Rotation)
        (Transformation|SetActorRotation (Math|Rotator|MakeRotator (.roll _basic_rotaion_3) (.pitch _basic_rotaion_3) (Math|Float|Lerp (Variables|CameraMovement|GetStart%20Routine) (Variables|CameraMovement|GetEnd%20Routine) (Variables|CameraMovement|GetCurrent%20Lerp))))
        (else
          (Transformation|SetActorRotation (Math|Rotator|MakeRotator (.roll _basic_rotaion) (.pitch _basic_rotaion) (Math|Float|Lerp (Variables|CameraMovement|GetEnd%20Routine) (Variables|CameraMovement|GetStart%20Routine) (Variables|CameraMovement|GetCurrent%20Lerp))))))
      (if (>= (Variables|CameraMovement|GetCurrent%20Lerp) 1.0)
        _))))

(event Custom|BackToRoutine
  ;[0 1 0.4134] Auto Rotation
  ;;[0 0.6366 1] Revient à sa routine quand le joueur est perdu de vu
  ;;;[0.8244 0.5491 1] Parametrage pour revenir correctement à la routine basique
  (Variables|CameraMovement|SetPrevious%20Self%20Rotation (Transformation|GetActorRotation))
  (Variables|CameraMovement|SetBackingToRoutine true))

(event Custom|SwitchOff
  ;[0 0 0] Switch On / Off
  (Variables|Fire|SetIs%20Off true)
  (Utilities|FlowControl|FlipFlop
    (:A
      (Rendering|Material|SetMaterial (Variables|Default|GetLight) 0 "/Game/Graphics/MI_EmissiveGrey.MI_EmissiveGrey"))
    (:B
      (Rendering|Material|SetMaterial (Variables|Default|GetLight) 0 "/Game/Graphics/MI_EmissiveGreen.MI_EmissiveGreen"))))

(event Custom|Component%20Parameter
  ;[0.1302 0.1302 0.1302] Enregistre la position de base de la tourelle pour la retrouver plus tard ou pour maintenir les components en place
  (bind _output_get (Variables|CameraMovement|SetBasic%20Rotaion (Transformation|GetActorRotation)))
  (Transformation|SetActorRotation (Math|Rotator|MakeRotator (.Roll (Math|Rotator|BreakRotator _output_get)) (.Pitch (Math|Rotator|BreakRotator _output_get)) (Variables|CameraMovement|GetStart%20Routine))))

(event Custom|ResetWindUp
  ;[1 0.9582 0] Event Tick
  (Utilities|FlowControl|DoOnce false ; enters at Reset
    (:Completed
      (Audio|PlaySoundatLocation 0 (Transformation|GetActorLocation) "0, 0, 0" 1.0 1.0 0.0 0 0 0 0))))

(event Custom|DontSeeDeltaTime
  (params (Delta%20Second :type Float%20%28double-precision%29))
  ;[0.4629 1 0] On See Pawn
  ;;[0.8131 1 0] Timer qui compte pendant combien de temps la tourelle ne voit personne (appelé dans l'Event Tick).
  (bind _output_get (Variables|Detection|SetDeltaTimeStandBy (+ Delta%20Second (Variables|Detection|GetDeltaTimeStandBy))))
  (if (> _output_get (Variables|Detection|GetTimeBeforeReturnToRoutine))
    (CallFunction|UnseePawn)))

(event Custom|Turret%20Sound
  ;[1 0.9582 0] Event Tick
  ;;[1 1 1] Son du Mouvement de la Tourelle
  (if (Variables|CameraMovement|GetMoving)
    (Utilities|FlowControl|DoOnce false
      (:Completed
        (bind _returnvalue (Audio|SpawnSoundatLocation 0 (Transformation|GetActorLocation) "0, 0, 0" 1.0 1.0 0.0 0 0))
        (Variables|Default|SetMovementSound _returnvalue)))
    (else
      (bind _movementsound (Variables|Default|GetMovementSound)
        (:then
          (Audio|Components|Audio|Stop _movementsound))
        (:else)))))

(event Custom|AlertsOthersTurrets
  (params (Target :type Actor%20Object%20Reference))
  ;[0.4629 1 0] On See Pawn
  ;;[0 1 0.6438] Alerte les tourelles qui lui sont lié lorsqu'elle voit quelqu'un
  (for _array_element (Variables|Fire|GetLinked%20Turrets)
    _))

(event Custom|Can%20Rotate
  ;[0 1 0.4134] Auto Rotation
  ;;[0.09842 1 0.1359] Vérifie si la tourelle peut se déplacer ou si elle est au bout de sa rotation
  (if (>= (Variables|CameraMovement|GetCurrent%20Lerp) 1.0)
    (if (Variables|CameraMovement|GetBackingToRoutine)
      (Variables|CameraMovement|SetBackingToRoutine false)
      (else
        (Utilities|FlowControl|Delay (Variables|CameraMovement|GetDelayBeforeSwitchRotation))
        (Variables|CameraMovement|SetNegate%20Rotation (not (Variables|CameraMovement|GetNegate%20Rotation)))))
    (Variables|CameraMovement|SetCurrent%20Lerp 0.0)
    (CallFunction|AutoRotation (Utilities|Time|GetWorldDeltaSeconds))
    (else
      (CallFunction|AutoRotation (Utilities|Time|GetWorldDeltaSeconds)))))

(event Custom|Follow%20Target
  ;[1 0 0.3159] Suit sa cible du regard (Appelé en Event Tick)
)

(event Custom|SwitchOn
  ;[0 0 0] Switch On / Off
  (Variables|Fire|SetIs%20Off false)
  (Utilities|FlowControl|FlipFlop
    (:A
      (Rendering|Material|SetMaterial (Variables|Default|GetLight) 0 "/Game/Graphics/MI_EmissiveGrey.MI_EmissiveGrey"))
    (:B
      (Rendering|Material|SetMaterial (Variables|Default|GetLight) 0 "/Game/Graphics/MI_EmissiveGreen.MI_EmissiveGreen"))))

(event Custom|UnseePawn
  ;[0.4629 1 0] On See Pawn
  ;;[1 0.4631 0] Quand la cible est perdue de vue
  ;;;[0.5729 0.05715 0] Vérification si plus aucune tourelle ne voit la cible.
)

(event Custom|SeePawn
  (params (TargetSeen :type Actor%20Object%20Reference))
  ;[0.4629 1 0] On See Pawn
  ;;[0 0.4253 1] Change la couleur du laser lorqu'elle à vu quelqu'un
  (Variables|Detection|SetIs%20Targeting true)
  (bind _output_get (Variables|Detection|SetTarget%20Seen TargetSeen))
  (CallFunction|AlertsOthersTurrets _output_get)
  (Variables|CameraMovement|SetMoving false)
  (Audio|PlaySoundatLocation 0 (Transformation|GetActorLocation) "0, 0, 0" 1.0 1.0 0.0 0 0 0 0))

(event EventBeginPlay
  (CallFunction|ComponentParameter))

(event EventTick
  (params (DeltaSeconds :type Float%20%28single-precision%29))
  (if (not (Variables|Fire|GetIs%20Off))
    (Utilities|FlowControl|Sequence
      (:then_0
        (if (Variables|Detection|GetIs%20Targeting)
          ;[1 0.9582 0] Event Tick
          (if (<= (Variables|Detection|GetDeltaTimeStandBy) (Variables|/Script/AIModule.PawnSensingComponent|GetSensingInterval (Variables|Default|GetPawnSensing)))
            (CallFunction|FollowTarget)
            (else
              (CallFunction|BacktoRoutine)))
          (else
            (CallFunction|CanRotate))))
      (:then_1
        (if (Variables|Detection|GetIs%20Targeting)
          (CallFunction|DontSeeDeltaTime DeltaSeconds))))))

(fn ConstructionScript)