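; BP_IAGuard is an enemy guard Blueprint that walks along the world X axis on a repeating loop.
; On BeginPlay it runs Move, which casts its controller to AIC_Enemy and issues an AI MoveTo 500 units from its current location.
; When a move finishes it waits two seconds and moves again, while French debug prints mark each branch, including a failed request or cast.
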(event Custom|Move
  (bind _asaic_enemy (Utilities|Casting|CastToAIC_Enemy (Pawn|GetController))
    (:then
      (AI|AIMoveTo _asaic_enemy (+ (Transformation|GetActorLocation) "500.000000,0.000000,0.000000") 0 -1.0 "Default" "Default" true true
        (:then
          (Development|PrintText "De ce côté"))
        (:OnRequestFailed
          (Development|PrintText "Par Là"))
        (:OnMoveFinished
          (Development|PrintText "Là")
          (Utilities|FlowControl|Delay 2.0)
          (CallFunction|Move))))
    (:CastFailed
      (Development|PrintText "Ici"))))

(event EventBeginPlay
  (CallFunction|Move))

(fn ConstructionScript)