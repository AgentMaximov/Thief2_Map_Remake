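; Enemy pawn Blueprint that links to its AIC_Enemy02 AI controller and sight-detection icon widget.
; BeginPlay requires a BP_GameMode, caches the controller and widget, and sets itself as the widget's owner.
; Tick only debug-draws a short forward trace whose result is unused.
; StartShooting and StopShooting are empty; the crouch-aware hitscan rifle, noise reporting, damage and game-mode enemy registration logic sit disconnected and never run.
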(event Custom|StartShooting)

(event Custom|StopShooting)

(event EventBeginPlay
  (bind _asbp_game_mode (Utilities|Casting|CastToBP_GameMode (Game|GetGameMode)))
  (bind _asaic_enemy_02 (Utilities|Casting|CastToAIC_Enemy02 (AI|GetAIController self)))
  (Variables|Default|SetAIC_REF _asaic_enemy_02)
  (bind _aswbp_sight_detection_icon (Utilities|Casting|CastToWBP_SightDetectionIcon (UserInterface|GetUserWidgetObject (Variables|Default|GetWidget))))
  (Variables|/Game/Blueprint/Enemis/EnemyAI/Widgets/WBP_SightDetectionIcon.WBP_SightDetectionIcon_C|SetPawnOwner _aswbp_sight_detection_icon self)
  (Variables|Default|SetSightDetectionIconREF _aswbp_sight_detection_icon))

(event EventTick
  (params (DeltaSeconds :type Float%20%28single-precision%29))
  (bind _returnvalue (Transformation|GetActorLocation))
  (Collision|LineTraceByChannel _returnvalue (+ _returnvalue (* (Math|Vector|GetForwardVector (Transformation|GetActorRotation)) 2e+02)) "TraceTypeQuery1" false 0 "ForOneFrame"))

(fn ConstructionScript)