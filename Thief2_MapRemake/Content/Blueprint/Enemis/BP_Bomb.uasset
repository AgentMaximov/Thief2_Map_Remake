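; BP_Bomb is an enemy-folder bomb actor that explodes on a timer after it spawns.
; After a configurable delay, the ShockWave timeline uniformly scales up the Explosion component, an emissive sphere, then destroys the actor.
; The Explosion overlap event, meant for damage, only casts to BP_PlayerCharacter and applies no damage yet.
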(event OnComponentBeginOverlap(Explosion)
  (params (OverlappedComponent :type Primitive%20Component%20Object%20Reference) (OtherActor :type Actor%20Object%20Reference) (OtherComp :type Primitive%20Component%20Object%20Reference) (OtherBodyIndex :type Integer) (bFromSweep :type Boolean) (SweepResult :type Hit%20Result%20Structure%20%28by%20ref%29))
  ;[0 1 0.2094] Appel pour les dégâts
  (Utilities|Casting|CastToBP_PlayerCharacter OtherActor))

(event Custom|Explosion!!!
  ;[1 0.3582 0.2865] L'explosion c'est juste une sphère qui grossit avec une texture emissive
  (Utilities|FlowControl|Delay (Variables|Default|GetTime%20Before%20Explosion))
  (bind _scale (Timeline|ShockWave PlayFromStart)
    (:Update
      (Transformation|SetWorldScale3D (Variables|Default|GetExplosion) (Math|Vector|MakeVector _scale _scale _scale)))
    (:Finished
      (Actor|DestroyActor))))

(event EventBeginPlay
  ;[1 1 1] Event Begin Play
  (CallFunction|Explosion!!!))

(fn ConstructionScript)