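; Enemy turret that shoots at the player when a camera reports seeing them, until it is destroyed.
; SeePlayer stores the target and starts a CanFire/FireProjectile loop, spawning the configured projectile at the muzzle and repeating after a fire-rate delay.
; Each shot first rotates the whole actor toward the target, then restores the Foot's saved world transform so the base stays fixed.
; UnseePlayer clears the target; Destroyed stops firing and toggles Body visibility.
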(event Custom|See%20Player
  (params (Player%20Target :type BP%20Player%20Character%20Object%20Reference))
  ;[0.3311 1 0.03269] Infos envoyées par la caméra
  (Variables|Default|SetPlayer%20Target Player%20Target)
  (Variables|Default|SetTargeting true)
  (CallFunction|CanFire))

(event Custom|Unsee%20Player
  ;[0.3311 1 0.03269] Infos envoyées par la caméra
  (Variables|Default|SetPlayer%20Target 0)
  (Variables|Default|SetTargeting false))

(event Custom|Fire%20Projectile
  (bind _muzzle (Variables|Default|GetMuzzle))
  ;[0.3021 0 0] Tire un projectile
  (if (Variables|Default|GetCan%20Fire)
    (Variables|Default|SetCan%20Fire false)
    (Game|SpawnActorfromClass (Variables|AParamétrer|GetTypeDeTire) (Math|Transform|MakeTransform (Transformation|GetWorldLocation _muzzle) (Transformation|GetWorldRotation _muzzle)) "AlwaysSpawn" "MultiplyWithRoot" 0 0)
    (Utilities|FlowControl|Delay (Variables|AParamétrer|GetFireRate))
    (Variables|Default|SetCan%20Fire true)
    (CallFunction|CanFire)))

(event Custom|CanFire
  (bind _player_target (Variables|Default|GetPlayer%20Target))
  ;[1 0.3 0] Vérifie si la tourelle peut tirer et si oui, se tourne vers la cible
  (if (not (Variables|Default|GetIs%20Destroyed))
    (Utilities|IsValid _player_target
      (:Is%20Valid
        (Transformation|SetActorRotation (Math|Rotator|FindLookatRotation (Transformation|GetActorLocation) (Transformation|GetActorLocation _player_target)))
        (Transformation|SetWorldTransform (Variables|Default|GetFoot) (Variables|Default|GetFoot%20World%20Transform) false false)
        (CallFunction|FireProjectile)))))

(event Custom|Destroyed
  ;[1 0 0.03761] Event Destroyed
  (Variables|Default|SetIs%20Destroyed true)
  (Rendering|ToggleVisibility (Variables|Default|GetBody) true))

(event EventBeginPlay
  ;[1 1 1] Event Begin Play
  ;;[0.0625 0.0625 0.0625 0.4] Enregistre la position du pied pour l'empêcher de bouger
  (Variables|Default|SetFoot%20World%20Transform (Transformation|GetWorldTransform (Variables|Default|GetFoot))))

(fn ConstructionScript)