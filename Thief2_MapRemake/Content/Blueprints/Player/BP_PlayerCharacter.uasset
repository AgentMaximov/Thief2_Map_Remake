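; BP_PlayerCharacter is the player character Blueprint, which tracks a light level value.
; On BeginPlay it caches the BP_GameMode, then the BP_PlayerController, and stops at the first failed cast.
; AdjustLightLevel takes a light source's level and raises LightLevel to it only if it is higher, with no reset or decrease in this Blueprint.
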(event EventBeginPlay
  (bind _asbp_game_mode (Utilities|Casting|CastToBP_GameMode (Game|GetGameMode)))
  (Variables|Default|SetGameMode _asbp_game_mode)
  (bind _asbp_player_controller (Utilities|Casting|CastToBP_PlayerController (Pawn|GetController)))
  (Variables|Default|SetPlayerController _asbp_player_controller))

(fn ConstructionScript)

(fn AdjustLightLevel
  (params (LightSourceLevel :type Float%20%28double-precision%29))
  (Variables|Light|SetLightLevel (Math|Float|SelectFloat LightSourceLevel (Variables|Light|GetLightLevel) (> LightSourceLevel (Variables|Light|GetLightLevel)))))