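; BP_Light is a point light actor that detects when BP_PlayerCharacter is within its range.
; On BeginPlay it sets the light's intensity and sizes its attenuation radius slightly inside the scaled DetectionCollision sphere.
; Sphere overlaps cache the player once and toggle PlayerInRange, which gates a debug-drawn visibility trace on Tick.
; The trace has no end point wired, and a distance-based brightness calculation using its hit result is left unused.
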(event OnComponentBeginOverlap(DetectionCollision)
  (params (OverlappedComponent :type Primitive%20Component%20Object%20Reference) (OtherActor :type Actor%20Object%20Reference) (OtherComp :type Primitive%20Component%20Object%20Reference) (OtherBodyIndex :type Integer) (bFromSweep :type Boolean) (SweepResult :type Hit%20Result%20Structure%20%28by%20ref%29))
  (bind _asbp_player_character (Utilities|Casting|CastToBP_PlayerCharacter OtherActor))
  (Utilities|FlowControl|Sequence
    (:then_0
      (Utilities|FlowControl|DoOnce false
        (:Completed
          (Variables|Default|SetPlayer _asbp_player_character))))
    (:then_1
      (Variables|Default|SetPlayerInRange true))))

(event OnComponentEndOverlap(DetectionCollision)
  (params (OverlappedComponent :type Primitive%20Component%20Object%20Reference) (OtherActor :type Actor%20Object%20Reference) (OtherComp :type Primitive%20Component%20Object%20Reference) (OtherBodyIndex :type Integer))
  (Utilities|Casting|CastToBP_PlayerCharacter OtherActor)
  (Variables|Default|SetPlayerInRange false))

(event EventBeginPlay
  (bind _detectioncollision (Variables|Default|GetDetectionCollision))
  (Rendering|Lighting|SetAttenuationRadius (Variables|Default|GetPointLight) (* (.z (Transformation|GetWorldScale _detectioncollision)) (Variables|/Script/Engine.SphereComponent|GetSphereRadius _detectioncollision) 0.9))
  (Rendering|Components|Light|SetIntensity (Variables|Default|GetPointLight) (Variables|Default|GetIntensity)))

(event EventTick
  (params (DeltaSeconds :type Float%20%28single-precision%29))
  (if (Variables|Default|GetPlayerInRange)
    (bind _outhit (Collision|LineTraceByChannel (Transformation|GetActorLocation) "0, 0, 0" "TraceTypeQuery1" false 0 "ForOneFrame" true "(R=0.993651,G=1.000000,B=0.967060,A=1.000000)"))))

(fn ConstructionScript)